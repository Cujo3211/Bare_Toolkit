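; Blueprint function library holding card abilities for a card game, such as drawing, cloning, stat and health boosts, damage and summoning from the deck.
; Each function takes the calling card and an ability index, using that ability's AbilityInt as magnitude or repeat count.
; Summons find a free placement, spawn and place cards through the owning player; cloning can fall back to random spots, deck spawns retry via MultiGate.
; Most abilities also send a message to the player's log.
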(fn Ability-DrawCard(s)
  (params (CallingCard :type 3D%20Card%20Object%20Reference) (AbilityIndex :type Integer))
  (bind _ability_struct_refs (Variables|/Game/CCGToolkit/Blueprints/Gameplay/3DCard.3DCard_C|GetAbility_Struct_Refs CallingCard))
  (bind _owningplayer (Variables|/Game/CCGToolkit/Blueprints/Gameplay/3DCard.3DCard_C|GetOwningPlayer CallingCard))
  (bind _item (Utilities|Array|Get(acopy) _ability_struct_refs AbilityIndex))
  (bind _ability_int (Utilities|Struct|BreakAbility_Struct _item))
  (Default|ServerDrawCard _owningplayer "None" "NewEnumerator0" false _ability_int)
  (Default|EventCreateDisplayMessage _owningplayer (CallFunction|PickupCard(s)LogMessage _ability_int) "(R=0.066667,G=1.000000,B=0.000000,A=1.000000)" false 0.0 true)
  (return))

(fn Ability-IncreaseAttack
  (params (CallingCard :type 3D%20Card%20Object%20Reference) (AbilityIndex :type Integer))
  (bind _ability_struct_refs (Variables|/Game/CCGToolkit/Blueprints/Gameplay/3DCard.3DCard_C|GetAbility_Struct_Refs CallingCard))
  (bind _item (Utilities|Array|Get(acopy) _ability_struct_refs AbilityIndex))
  (bind _ability_int (Utilities|Struct|BreakAbility_Struct _item))
  (Default|EventCreateDisplayMessage (Variables|/Game/CCGToolkit/Blueprints/Gameplay/3DCard.3DCard_C|GetOwningPlayer CallingCard) (CallFunction|IncreaseAttackLogMessage (Variables|/Game/CCGToolkit/Blueprints/Gameplay/3DCard.3DCard_C|GetName CallingCard) _ability_int) "(R=0.069650,G=1.000000,B=0.000000,A=1.000000)" false 0.0 true)
  (Variables|/Game/CCGToolkit/Blueprints/Gameplay/3DCard.3DCard_C|SetAttack CallingCard (+ (Variables|/Game/CCGToolkit/Blueprints/Gameplay/3DCard.3DCard_C|GetAttack CallingCard) _ability_int))
  (Default|MulticastUpdateVisualStats CallingCard)
  (return))

(fn Ability-CloneCard
  (params (CallingCard :type 3D%20Card%20Object%20Reference) (AbilityIndex :type Integer) (RandomPlacement :type Boolean))
  (bind _ability_struct_refs (Variables|/Game/CCGToolkit/Blueprints/Gameplay/3DCard.3DCard_C|GetAbility_Struct_Refs CallingCard))
  (bind _owningplayer (Variables|/Game/CCGToolkit/Blueprints/Gameplay/3DCard.3DCard_C|GetOwningPlayer CallingCard))
  (bind _carddatatablename (Variables|/Game/CCGToolkit/Blueprints/Gameplay/3DCard.3DCard_C|GetCardDataTableName CallingCard))
  (bind _placementowner (Variables|/Game/CCGToolkit/Blueprints/Gameplay/3DCard.3DCard_C|GetPlacementOwner CallingCard))
  (bind _item (Utilities|Array|Get(acopy) _ability_struct_refs AbilityIndex))
  (bind (_returnplacement _returnvalid) (CallFunction|GetClosestAvailablePlacement _placementowner _carddatatablename "NewEnumerator0"))
  (bind _ability_int (Utilities|Struct|BreakAbility_Struct _item))
  (Default|EventCreateDisplayMessage _owningplayer (CallFunction|CloneCardLogMessage (Variables|/Game/CCGToolkit/Blueprints/Gameplay/3DCard.3DCard_C|GetName CallingCard) _ability_int) "(R=0.066667,G=1.000000,B=0.000000,A=1.000000)" false 0.0 true)
  (Utilities|FlowControl|ForLoopwithBreak 1 _ability_int
    (:LoopBody
      (if RandomPlacement :!label _label ; Choose Random Available Placement on the board?
        (bind (_returnarray _validplacements) (CallFunction|GetPlayersAvailablePlacements _owningplayer false :!label _label_2))
        (if _validplacements
          (LocalVariables|SetGoalPlacement (Utilities|Array|Get(acopy) _returnarray (Math|Random|RandomIntegerinRange 0 (- (Utilities|Array|Length _returnarray) 1))))
          (else
            (Development|PrintString 0 "No Avaliable Spots to Clone" false true "(R=0.770000,G=0.000000,B=0.049357,A=1.000000)" 1e+01)
            (return)))
        (elif _returnvalid
          (LocalVariables|SetGoalPlacement _returnplacement)
          (else
            (goto _label_2))))
      (Utilities|IsValid (LocalVariables|GetGoalPlacement)
        (:Is%20Valid
          (bind _card_created (Default|CreatePlaceableCard(Server) _owningplayer (Variables|/Game/CCGToolkit/Blueprints/Gameplay/3DCard.3DCard_C|GetCardDataTableName CallingCard) (Variables|/Game/CCGToolkit/Blueprints/Gameplay/3DCard.3DCard_C|GetCardSet CallingCard) (|IncreaseSpawnHeightFromSummoningCard_2 CallingCard)))
          (bind _returncard (Default|SetCustomCardData _owningplayer _card_created false))
          (Default|PlaceCardonBoard _owningplayer _returncard (LocalVariables|GetGoalPlacement)))
        (:Is%20Not%20Valid
          (goto _label))))
    (:Completed
      (return))))

(fn Ability-IncreasePlayerHealth
  (params (CallingCard :type 3D%20Card%20Object%20Reference) (AbilityIndex :type Integer))
  (bind _ability_struct_refs (Variables|/Game/CCGToolkit/Blueprints/Gameplay/3DCard.3DCard_C|GetAbility_Struct_Refs CallingCard))
  (bind _owningplayer (Variables|/Game/CCGToolkit/Blueprints/Gameplay/3DCard.3DCard_C|GetOwningPlayer CallingCard))
  (bind _item (Utilities|Array|Get(acopy) _ability_struct_refs AbilityIndex))
  (bind _ability_int (Utilities|Struct|BreakAbility_Struct _item))
  (Default|IncreasePlayerHealth _owningplayer _ability_int)
  (Default|EventCreateDisplayMessage _owningplayer (Utilities|String|Append "Players health Increased by + " (Utilities|String|ToString(Integer) _ability_int)) "(R=0.066667,G=1.000000,B=0.000000,A=1.000000)" false 0.0 true)
  (return))

(fn Ability-DealRetaliationDamage
  (params (Calling%20Card :type 3D%20Card%20Object%20Reference) (AbilityIndex :type Integer))
  (bind _ability_struct_refs (Variables|/Game/CCGToolkit/Blueprints/Gameplay/3DCard.3DCard_C|GetAbility_Struct_Refs Calling%20Card))
  (bind _item (Utilities|Array|Get(acopy) _ability_struct_refs AbilityIndex))
  (bind _ability_int (Utilities|Struct|BreakAbility_Struct _item))
  (if (Utilities|IsValid (Variables|/Game/CCGToolkit/Blueprints/Gameplay/3DCard.3DCard_C|GetDamageDealingCard_Ref Calling%20Card)) ; Is there a valid Dealing card to retaliate to? If there is no Dealing card, it is possible that the last damage taken does not allow Retliate.
    (Default|EventCreateDisplayMessage (Variables|/Game/CCGToolkit/Blueprints/Gameplay/3DCard.3DCard_C|GetOwningPlayer Calling%20Card) (Utilities|String|Append (Utilities|String|ToString(Text) (Variables|/Game/CCGToolkit/Blueprints/Gameplay/3DCard.3DCard_C|GetName Calling%20Card)) "  dealing  '" (Utilities|String|ToString(Integer) _ability_int) "'  retaliation damage to  " (Utilities|String|ToString(Text) (Variables|/Game/CCGToolkit/Blueprints/Gameplay/3DCard.3DCard_C|GetName (Variables|/Game/CCGToolkit/Blueprints/Gameplay/3DCard.3DCard_C|GetDamageDealingCard_Ref Calling%20Card)))) "(R=1.000000,G=0.439106,B=0.000000,A=1.000000)" false 0.0 true)
    (CallFunction|DealDamagetoCard (Variables|/Game/CCGToolkit/Blueprints/Gameplay/3DCard.3DCard_C|GetDamageDealingCard_Ref Calling%20Card) 0 _ability_int Calling%20Card)
    (Variables|/Game/CCGToolkit/Blueprints/Gameplay/3DCard.3DCard_C|SetDamageDealingCard_Ref Calling%20Card 0)))

(fn Ability-DamageAllCardsonBoard
  (params (CallingCard :type 3D%20Card%20Object%20Reference) (AbilityIndex :type Integer))
  (bind _outactors (Actor|GetAllActorsOfClass 0 "/Game/CCGToolkit/Blueprints/Gameplay/3DCard.3DCard_C"))
  (for _array_element _outactors
    (if (not (== _array_element CallingCard)) ; Does the card in array equal the card the calling card?
      (if (not (Variables|/Game/CCGToolkit/Blueprints/Gameplay/3DCard.3DCard_C|GetbInGraveyard _array_element)) ; is the Card in the graveyard
        (if (Variables|/Game/CCGToolkit/Blueprints/Gameplay/3DCard.3DCard_C|GetbIsPlaced _array_element) ; Is the card currently placed on the board?
          (CallFunction|DealDamagetoCard _array_element 0 (.Ability_Int (Utilities|Struct|BreakAbility_Struct (Utilities|Array|Get(acopy) (Variables|/Game/CCGToolkit/Blueprints/Gameplay/3DCard.3DCard_C|GetAbility_Struct_Refs CallingCard) AbilityIndex))))))))
  (return))

(fn Ability-SpawnRandomCard(s)fromDeck
  (params (CallingCard :type 3D%20Card%20Object%20Reference) (AbilityIndex :type Integer))
  (bind _placementowner (Variables|/Game/CCGToolkit/Blueprints/Gameplay/3DCard.3DCard_C|GetPlacementOwner CallingCard))
  (bind _ability_struct_refs (Variables|/Game/CCGToolkit/Blueprints/Gameplay/3DCard.3DCard_C|GetAbility_Struct_Refs CallingCard))
  (bind _owningplayer (Variables|/Game/CCGToolkit/Blueprints/Gameplay/3DCard.3DCard_C|GetOwningPlayer CallingCard))
  (bind _item (Utilities|Array|Get(acopy) _ability_struct_refs AbilityIndex))
  (bind _ability_int (Utilities|Struct|BreakAbility_Struct _item))
  (Default|EventCreateDisplayMessage _owningplayer (Utilities|String|Append (Utilities|String|ToString(Text) (Variables|/Game/CCGToolkit/Blueprints/Gameplay/3DCard.3DCard_C|GetName CallingCard)) " Cloned up to + " (Utilities|String|ToString(Integer) _ability_int) " Times!") "(R=0.066667,G=1.000000,B=0.000000,A=1.000000)" false 0.0 true)
  (LocalVariables|SetInitialGoalPlacement _placementowner)
  (Utilities|FlowControl|ForLoopwithBreak 1 _ability_int :!label _label
    (:LoopBody
      (bind (_card _cardrace _index) (CallFunction|GetRandomCardfromDeck _owningplayer :!label _label_2))
      (if (.ReturnValid (CallFunction|GetClosestAvailablePlacement _placementowner _card "NewEnumerator0"))
        (bind _output_get (LocalVariables|SetGoalPlacement (.ReturnPlacement (CallFunction|GetClosestAvailablePlacement _placementowner _card "NewEnumerator0"))))
        (Utilities|IsValid _output_get
          (:Is%20Valid
            (bind _card_created (Default|CreatePlaceableCard(Server) _owningplayer _card _cardrace (|IncreaseSpawnHeightFromSummoningCard_2_2 CallingCard)))
            (bind _returncard (Default|SetCustomCardData _owningplayer _card_created true))
            (Default|PlaceCardonBoard _owningplayer _returncard (LocalVariables|GetGoalPlacement))
            (CallFunction|RemoveCardfromDeck _owningplayer false _index))
          (:Is%20Not%20Valid
            (goto _label Break)))
        (else
          (Utilities|FlowControl|MultiGate false false -1
            (:Out%200
              (goto _label_2))
            (:Out%201
              (goto _label_2))
            (:Out%202
              (goto _label_2))
            (:Out%203
              (goto _label_2))
            (:Out%204
              (goto _label Break))))))
    (:Completed
      (return))))

(fn Ability-GiveTurnPointstoAllActiveCards
  (params (CallingCard :type 3D%20Card%20Object%20Reference) (PlayerController :type Card%20Game%20Player%20Controller%20Object%20Reference) (AbilityIndex :type Integer))
  (bind _ability_struct_refs (Variables|/Game/CCGToolkit/Blueprints/Gameplay/3DCard.3DCard_C|GetAbility_Struct_Refs CallingCard))
  (bind _owningplayer (Variables|/Game/CCGToolkit/Blueprints/Gameplay/3DCard.3DCard_C|GetOwningPlayer CallingCard))
  (bind _item (Utilities|Array|Get(acopy) _ability_struct_refs AbilityIndex))
  (bind _ability_int (Utilities|Struct|BreakAbility_Struct _item))
  (for _array_element (Variables|/Game/CCGToolkit/Blueprints/CardGamePlayerController.CardGamePlayerController_C|GetCardsOnBoard _owningplayer)
    (Variables|/Game/CCGToolkit/Blueprints/Gameplay/3DCard.3DCard_C|SetTurnPoints _array_element (+ (Variables|/Game/CCGToolkit/Blueprints/Gameplay/3DCard.3DCard_C|GetTurnPoints _array_element) _ability_int))
    (Default|MulticastUpdateCardVisual _array_element true))
  (Default|EventCreateDisplayMessage _owningplayer (Utilities|String|Append "All Cards have gained  +" (Utilities|String|ToString(Integer) _ability_int) " Turn Points! ") "(R=0.066667,G=1.000000,B=0.000000,A=1.000000)" false 0.0 true)
  (return))

(fn Ability-IncreaseTurnPoints
  (params (CallingCard :type 3D%20Card%20Object%20Reference) (AbilityIndex :type Integer))
  (Variables|/Game/CCGToolkit/Blueprints/Gameplay/3DCard.3DCard_C|SetTurnPoints CallingCard (+ (Variables|/Game/CCGToolkit/Blueprints/Gameplay/3DCard.3DCard_C|GetTurnPoints CallingCard) (.Ability_Int (Utilities|Struct|BreakAbility_Struct (Utilities|Array|Get(acopy) (Variables|/Game/CCGToolkit/Blueprints/Gameplay/3DCard.3DCard_C|GetAbility_Struct_Refs CallingCard) AbilityIndex))))))