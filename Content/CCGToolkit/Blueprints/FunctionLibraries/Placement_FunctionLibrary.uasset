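; Blueprint function library for the card game's board placements, finding open slots and checking whether a card can go in one.
; Available-placement lookup gathers non-full CardPlacement actors that are shared (index 0) or owned by the player or opponent.
; Closest-slot search walks up to five linked neighbours left and right using random FlipFlops and MultiGates, validating card type and fullness.
; GetIsPlacementAvailable returns IsFull uninverted, so true means full.
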(fn GetPlayersAvailablePlacements
  (params (PlayerController :type Card%20Game%20Player%20Controller%20Object%20Reference) (Opponent :type Boolean))
  (bind _temp_boardplacement_array (LocalVariables|GetTemp_BoardPlacement_Array))
  (Utilities|Array|Clear (LocalVariables|GetTemp_BoardPlacement_Array))
  (bind (_selfplayer _oppenent) (CallFunction|GetPlayerStateReference PlayerController))
  (bind _ascard_game_player_state (Utilities|Casting|CastToCardGamePlayerState (select Opponent _oppenent _selfplayer))
    (:then
      (bind _outactors (Actor|GetAllActorsOfClass 0 "/Game/CCGToolkit/Blueprints/Gameplay/CardPlacement.CardPlacement_C"))
      (for _array_element _outactors
        (if (or (== (Variables|/Game/CCGToolkit/Blueprints/Gameplay/CardPlacement.CardPlacement_C|GetPlayerIndex _array_element) 0) (== (Variables|/Game/CCGToolkit/Blueprints/Gameplay/CardPlacement.CardPlacement_C|GetPlayerIndex _array_element) (Variables|/Game/CCGToolkit/Blueprints/CardGamePlayerState.CardGamePlayerState_C|GetCardGamePlayerId _ascard_game_player_state)))
          (if (not (Variables|/Game/CCGToolkit/Blueprints/Gameplay/CardPlacement.CardPlacement_C|GetbIsFull _array_element))
            (Utilities|Array|Add (LocalVariables|GetTemp_BoardPlacement_Array) _array_element))))
      (if (> (Utilities|Array|Length (LocalVariables|GetTemp_BoardPlacement_Array)) 0)
        (return _temp_boardplacement_array true)
        (else
          _)))
    (:CastFailed
      _))
  (return _temp_boardplacement_array false))

(fn GetClosestAvailablePlacement
  (params (Placement :type Card%20Placement%20Object%20Reference) (CardName :type Name) (CardSet :type CardSet_Enum%20Enum))
  (bind _placementleft (Variables|/Game/CCGToolkit/Blueprints/Gameplay/CardPlacement.CardPlacement_C|GetPlacementLeft Placement))
  (bind _placementleft_2 (Variables|/Game/CCGToolkit/Blueprints/Gameplay/CardPlacement.CardPlacement_C|GetPlacementLeft Placement))
  (bind _placementleft_3 (Variables|/Game/CCGToolkit/Blueprints/Gameplay/CardPlacement.CardPlacement_C|GetPlacementLeft Placement))
  (bind _placementleft_4 (Variables|/Game/CCGToolkit/Blueprints/Gameplay/CardPlacement.CardPlacement_C|GetPlacementLeft Placement))
  (bind _placementleft_5 (Variables|/Game/CCGToolkit/Blueprints/Gameplay/CardPlacement.CardPlacement_C|GetPlacementLeft Placement))
  (bind _placementright (Variables|/Game/CCGToolkit/Blueprints/Gameplay/CardPlacement.CardPlacement_C|GetPlacementRight Placement))
  (bind _placementright_2 (Variables|/Game/CCGToolkit/Blueprints/Gameplay/CardPlacement.CardPlacement_C|GetPlacementRight Placement))
  (bind _placementright_3 (Variables|/Game/CCGToolkit/Blueprints/Gameplay/CardPlacement.CardPlacement_C|GetPlacementRight Placement))
  (bind _placementright_4 (Variables|/Game/CCGToolkit/Blueprints/Gameplay/CardPlacement.CardPlacement_C|GetPlacementRight Placement))
  (bind _placementright_5 (Variables|/Game/CCGToolkit/Blueprints/Gameplay/CardPlacement.CardPlacement_C|GetPlacementRight Placement))
  (bind _placementleft_6 (Variables|/Game/CCGToolkit/Blueprints/Gameplay/CardPlacement.CardPlacement_C|GetPlacementLeft _placementleft_3))
  (bind _placementleft_7 (Variables|/Game/CCGToolkit/Blueprints/Gameplay/CardPlacement.CardPlacement_C|GetPlacementLeft _placementleft_4))
  (bind _placementleft_8 (Variables|/Game/CCGToolkit/Blueprints/Gameplay/CardPlacement.CardPlacement_C|GetPlacementLeft _placementleft_5))
  (bind _placementleft_9 (Variables|/Game/CCGToolkit/Blueprints/Gameplay/CardPlacement.CardPlacement_C|GetPlacementLeft _placementleft_2))
  (bind _placementright_6 (Variables|/Game/CCGToolkit/Blueprints/Gameplay/CardPlacement.CardPlacement_C|GetPlacementRight _placementright_2))
  (bind _placementright_7 (Variables|/Game/CCGToolkit/Blueprints/Gameplay/CardPlacement.CardPlacement_C|GetPlacementRight _placementright_3))
  (bind _placementright_8 (Variables|/Game/CCGToolkit/Blueprints/Gameplay/CardPlacement.CardPlacement_C|GetPlacementRight _placementright_4))
  (bind _placementright_9 (Variables|/Game/CCGToolkit/Blueprints/Gameplay/CardPlacement.CardPlacement_C|GetPlacementRight _placementright_5))
  (bind _placementleft_10 (Variables|/Game/CCGToolkit/Blueprints/Gameplay/CardPlacement.CardPlacement_C|GetPlacementLeft _placementleft_7))
  (bind _placementleft_11 (Variables|/Game/CCGToolkit/Blueprints/Gameplay/CardPlacement.CardPlacement_C|GetPlacementLeft _placementleft_8))
  (bind _placementleft_12 (Variables|/Game/CCGToolkit/Blueprints/Gameplay/CardPlacement.CardPlacement_C|GetPlacementLeft _placementleft_9))
  (bind _placementright_10 (Variables|/Game/CCGToolkit/Blueprints/Gameplay/CardPlacement.CardPlacement_C|GetPlacementRight _placementright_6))
  (bind _placementright_11 (Variables|/Game/CCGToolkit/Blueprints/Gameplay/CardPlacement.CardPlacement_C|GetPlacementRight _placementright_8))
  (bind _placementright_12 (Variables|/Game/CCGToolkit/Blueprints/Gameplay/CardPlacement.CardPlacement_C|GetPlacementRight _placementright_9))
  (bind _placementleft_13 (Variables|/Game/CCGToolkit/Blueprints/Gameplay/CardPlacement.CardPlacement_C|GetPlacementLeft _placementleft_10))
  (bind _placementleft_14 (Variables|/Game/CCGToolkit/Blueprints/Gameplay/CardPlacement.CardPlacement_C|GetPlacementLeft _placementleft_12))
  (bind _placementright_13 (Variables|/Game/CCGToolkit/Blueprints/Gameplay/CardPlacement.CardPlacement_C|GetPlacementRight _placementright_12))
  (bind _placementright_14 (Variables|/Game/CCGToolkit/Blueprints/Gameplay/CardPlacement.CardPlacement_C|GetPlacementRight _placementright_11))
  (bind _placementleft_15 (Variables|/Game/CCGToolkit/Blueprints/Gameplay/CardPlacement.CardPlacement_C|GetPlacementLeft _placementleft_14))
  (bind _placementright_15 (Variables|/Game/CCGToolkit/Blueprints/Gameplay/CardPlacement.CardPlacement_C|GetPlacementRight _placementright_14))
  (LocalVariables|SetLeftValidPath true)
  (LocalVariables|SetRightValidPath true)
  (Utilities|FlowControl|ForLoopwithBreak 0 12 :!label _label ; Check is 10 layers deep
    (:LoopBody
      (if (Math|Random|RandomBool)
        (Utilities|FlowControl|FlipFlop
          (:A
            (if (LocalVariables|GetLeftValidPath) :!label _label_2
              (Utilities|FlowControl|MultiGate false false -1
                (:Out%200
                  (bind (_isvalid _validplacement) (CallFunction|GetIsValidPlacement Placement CardName CardSet))
                  (if _isvalid
                    (if _validplacement
                      (LocalVariables|SetChosenPlacement Placement)
                      (goto _label Break))
                    (else
                      (LocalVariables|SetLeftValidPath false :!label _label_3))))
                (:Out%201
                  (bind (_isvalid_2 _validplacement_2) (CallFunction|GetIsValidPlacement _placementleft CardName CardSet))
                  (if _isvalid_2
                    (if _validplacement_2
                      (LocalVariables|SetChosenPlacement _placementleft)
                      (goto _label Break))
                    (else
                      (goto _label_3))))
                (:Out%202
                  (bind (_isvalid_3 _validplacement_3) (CallFunction|GetIsValidPlacement _placementleft_6 CardName CardSet))
                  (if _isvalid_3
                    (if _validplacement_3
                      (LocalVariables|SetChosenPlacement _placementleft_6)
                      (goto _label Break))
                    (else
                      (goto _label_3))))
                (:Out%203
                  (bind (_isvalid_4 _validplacement_4) (CallFunction|GetIsValidPlacement _placementleft_11 CardName CardSet))
                  (if _isvalid_4
                    (if _validplacement_4
                      (LocalVariables|SetChosenPlacement _placementleft_11)
                      (goto _label Break))
                    (else
                      (goto _label_3))))
                (:Out%204
                  (bind (_isvalid_5 _validplacement_5) (CallFunction|GetIsValidPlacement _placementleft_13 CardName CardSet))
                  (if _isvalid_5
                    (if _validplacement_5
                      (LocalVariables|SetChosenPlacement _placementleft_13)
                      (goto _label Break))
                    (else
                      (goto _label_3))))
                (:Out%205
                  (bind (_isvalid_6 _validplacement_6) (CallFunction|GetIsValidPlacement _placementleft_15 CardName CardSet))
                  (if _isvalid_6
                    (if _validplacement_6
                      (LocalVariables|SetChosenPlacement _placementleft_15)
                      (goto _label Break))
                    (else
                      (goto _label_3)))))
              (else
                (if (LocalVariables|GetRightValidPath) :!label _label_4
                  (Utilities|FlowControl|MultiGate false false -1
                    (:Out%200
                      (bind (_isvalid_7 _validplacement_7) (CallFunction|GetIsValidPlacement Placement CardName CardSet))
                      (if _isvalid_7
                        (if _validplacement_7
                          (LocalVariables|SetChosenPlacement Placement)
                          (goto _label Break))))
                    (:Out%201
                      (bind (_isvalid_8 _validplacement_8) (CallFunction|GetIsValidPlacement _placementright CardName CardSet))
                      (if _isvalid_8
                        (if _validplacement_8
                          (LocalVariables|SetChosenPlacement _placementright)
                          (goto _label Break))
                        (else
                          (LocalVariables|SetRightValidPath false :!label _label_5))))
                    (:Out%202
                      (bind (_isvalid_9 _validplacement_9) (CallFunction|GetIsValidPlacement _placementright_7 CardName CardSet))
                      (if _isvalid_9
                        (if _validplacement_9
                          (LocalVariables|SetChosenPlacement _placementright_7)
                          (goto _label Break))
                        (else
                          (goto _label_5))))
                    (:Out%203
                      (bind (_isvalid_10 _validplacement_10) (CallFunction|GetIsValidPlacement _placementright_10 CardName CardSet))
                      (if _isvalid_10
                        (if _validplacement_10
                          (LocalVariables|SetChosenPlacement _placementright_10)
                          (goto _label Break))
                        (else
                          (goto _label_5))))
                    (:Out%204
                      (bind (_isvalid_11 _validplacement_11) (CallFunction|GetIsValidPlacement _placementright_13 CardName CardSet))
                      (if _isvalid_11
                        (if _validplacement_11
                          (LocalVariables|SetChosenPlacement _placementright_13)
                          (goto _label Break))
                        (else
                          (goto _label_5))))
                    (:Out%205
                      (bind (_isvalid_12 _validplacement_12) (CallFunction|GetIsValidPlacement _placementright_15 CardName CardSet))
                      (if _isvalid_12
                        (if _validplacement_12
                          (LocalVariables|SetChosenPlacement _placementright_15)
                          (goto _label Break))
                        (else
                          (goto _label_5)))))
                  (elif (LocalVariables|GetLeftValidPath)
                    (goto _label_2)
                    (else
                      (return (LocalVariables|GetChosenPlacement) (Utilities|IsValid (LocalVariables|GetChosenPlacement)))))))))
          (:B
            (goto _label_4)))
        (else
          (Utilities|FlowControl|FlipFlop
            (:A
              (goto _label_4))
            (:B
              (goto _label_2))))))
    (:Completed
      (return (LocalVariables|GetChosenPlacement) (Utilities|IsValid (LocalVariables|GetChosenPlacement))))))

(fn GetIsPlacementAvailable
  (params (Placement :type Card%20Placement%20Object%20Reference))
  (return (Variables|/Game/CCGToolkit/Blueprints/Gameplay/CardPlacement.CardPlacement_C|GetbIsFull Placement)))

(fn GetIsValidPlacement
  (params (Placement :type Card%20Placement%20Object%20Reference) (CardName :type Name) (CardSet :type CardSet_Enum%20Enum))
  (bind _returnvalue (Utilities|IsValid Placement))
  (bind (_playerindex _ismulticardplacement _isfull _cardsinplacement _maxcardsinplacement _supportallcardtypes _validcardtypesarray) (Default|GetPlacementState Placement))
  (if _returnvalue
    (bind _datatable (CallFunction|GetCardData CardName CardSet))
    (if (>= (Utilities|Array|FindItem _validcardtypesarray (.Type (Utilities|Struct|BreakCard_Struct _datatable))) 0)
      (return _returnvalue (and (not _isfull) (>= (Utilities|Array|FindItem _validcardtypesarray (.Type (Utilities|Struct|BreakCard_Struct _datatable))) 0)))
      (else
        _)))
  (return false false))