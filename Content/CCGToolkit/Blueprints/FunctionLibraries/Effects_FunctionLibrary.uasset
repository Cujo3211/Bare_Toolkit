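; Effects function library for the card game toolkit that looks up and plays particle and sound effects.
; The card lookup maps a state to assets in the card struct, using a wildcard index for abilities; health-change states are left empty.
; The player lookup has all states unassigned.
; The spawn helper places a scaled emitter at a location or overriding actor's position and plays the sound in 2D, skipping invalid assets.
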(fn `Get Card Effects for State`
  (params (Effect :type "/Game/CCGToolkit/Blueprints/Enums/Effects_Enums/CardEffects_Enum Enum") (CardStruct :type "/Game/CCGToolkit/CardGame/Structs/Card_Struct Structure") (WildcardIndex :type Integer))
  (returns (Particle :type "ParticleSystem Object Reference") (SoundCue :type "SoundCue Object Reference"))
  (bind (_name _class _type _leader _visual _attack _health _abilities _description _placement_settings) (break `/Game/CCGToolkit/CardGame/Structs/Card_Struct` CardStruct))
  (bind (_damage _power _canattackplayer _canattackcards _combo_power _attack_particle _attack_soundcue) (break `/Game/CCGToolkit/CardGame/Structs/Attack_Struct` _attack))
  (bind (_health_2 _life_expectancy _dealth_particle _sound_cue_death) (break `/Game/CCGToolkit/CardGame/Structs/Health_Struct` _health))
  (bind (_owner _mana_cost _entry_particle _entry_soundcue) (break `/Game/CCGToolkit/CardGame/Structs/Placement_Struct` _placement_settings))
  (bind (_type_2 _ability_int _trigger _after_use_state _particle _soundcue) (break `/Game/CCGToolkit/CardGame/Structs/Ability_Struct` (`KismetArrayLibrary.Array_Get` _abilities WildcardIndex)))
  (return (select `/Game/CCGToolkit/Blueprints/Enums/Effects_Enums/CardEffects_Enum` Effect :`NewEnumerator0` _entry_particle :`NewEnumerator4` _attack_particle :`NewEnumerator3` _particle :`NewEnumerator5` _dealth_particle) (select `/Game/CCGToolkit/Blueprints/Enums/Effects_Enums/CardEffects_Enum` Effect :`NewEnumerator0` _entry_soundcue :`NewEnumerator4` _attack_soundcue :`NewEnumerator3` _soundcue :`NewEnumerator5` _sound_cue_death)))

(fn `Get Player Effects for State`
  (params (Effect :type "/Game/CCGToolkit/Blueprints/Enums/Effects_Enums/BoardPlayerEffects_Enum Enum"))
  (returns (Particle :type "ParticleSystem Object Reference") (SoundCue :type "SoundCue Object Reference"))
  (return (select `/Game/CCGToolkit/Blueprints/Enums/Effects_Enums/BoardPlayerEffects_Enum` Effect :!type "ParticleSystem Object Reference") (select `/Game/CCGToolkit/Blueprints/Enums/Effects_Enums/BoardPlayerEffects_Enum` Effect :!type "SoundCue Object Reference")))

(fn `Spawn Particle and Sound Effects`
  (params (ParticleToSpawn :type "ParticleSystem Object Reference") (Location :type "Vector Structure") (`OR ActorForLocation` :type "Actor Object Reference") (Scale :type "Vector Structure") (bAutoDestroy :type Boolean) (SoundCueToSpwn :type "SoundCue Object Reference") (Volume :type "Float (double-precision)"))
  (`/Engine/EditorBlueprintResources/StandardMacros.IsValid` ParticleToSpawn
    (:`Is Valid`
      (bind _returnvalue (`GameplayStatics.SpawnEmitterAtLocation` null ParticleToSpawn (select `bool` (`KismetSystemLibrary.IsValid` `OR ActorForLocation`) :`false` Location :`true` (`Actor.K2_GetActorLocation` `OR ActorForLocation`)) (struct) bAutoDestroy))
      (`SceneComponent.SetWorldScale3D` _returnvalue Scale))
    (:`Is Not Valid`
      _))
  (`/Engine/EditorBlueprintResources/StandardMacros.IsValid` SoundCueToSpwn
    (:`Is Valid`
      (`GameplayStatics.SpawnSound2D` null SoundCueToSpwn Volume))
    (:`Is Not Valid`
      _))
  (return))